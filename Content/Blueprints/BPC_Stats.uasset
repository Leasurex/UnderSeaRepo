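; BPC_Stats is a stats component that tracks Health and Charge for its owning actor.
; IncreaseValue and IncreaseCharge add a value to the matching stat, clamp it between zero and its max, then update an optional, externally assigned progress bar.
; Zero health triggers Death, which sends DeathMessage to the owner through the BPI_Damage interface.
; Zero charge only prints "No Charge".
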(event `Death`
  ;[0.05127 0.05127 0.05127] Send die message to the owner of this component. Owner needs to have the blueprint interface "BPI_Damage"
  (message `/Game/Blueprints/BPI_Damage.Death` (`self.GetOwner`)))

(event `SetHealthProgressBar`
  (params (HealthProgressBar :type "ProgressBar Object Reference"))
  ;[0.05127 0.05127 0.05127] HP bar
  (set `self.HealthProgressBar` HealthProgressBar))

(event `SetChargeProgressBar`
  (params (ChargeProgressBar :type "ProgressBar Object Reference"))
  ;[0.05127 0.05127 0.05127] Charge Bar
  (set `self.ChargeProgressBar` ChargeProgressBar))

(fn `IncreaseCharge`
  (params (Stat :type "/Game/Blueprints/E_Stats Enum" :default "NewEnumerator0") (Value :type "Float (double-precision)"))
  (switch `/Game/Blueprints/E_Stats` Stat
    (:`NewEnumerator1`
      ;[0.05127 0.05127 0.05127] Increase health by a "value" amount, capped at max
      (set `self.Charge` (`KismetMathLibrary.FClamp` (+ (`self.Charge`) Value) 0.0 (`self.MaxCharge`)))
      (`|ExecutionSequence`
        (:`then_0`
          ;[0.05127 0.05127 0.05127] Call No Charge!
          (if (<= (`self.Charge`) 0.0)
            (`KismetSystemLibrary.PrintString` "No Charge")))
        (:`then_1`
          ;[0.05127 0.05127 0.05127] Set percentage on Charge bar, check if there is a progress bar on the owner first
          (bind _chargeprogressbar (`self.ChargeProgressBar`)
            (:`then`
              (`ProgressBar.SetPercent` _chargeprogressbar (/ (`self.Charge`) (`self.MaxCharge`))))
            (:`else`)))))))

(fn `IncreaseValue`
  (params (Stat :type "/Game/Blueprints/E_Stats Enum" :default "NewEnumerator0") (Value :type "Float (double-precision)"))
  (switch `/Game/Blueprints/E_Stats` Stat
    (:`NewEnumerator0`
      ;[0.05127 0.05127 0.05127] Increase health by a "value" amount, capped at max
      (set `self.Health` (`KismetMathLibrary.FClamp` (+ (`self.Health`) Value) 0.0 (`self.MaxHealth`)))
      (`|ExecutionSequence`
        (:`then_0`
          ;[0.05127 0.05127 0.05127] Call Death function in this event graph
          (if (<= (`self.Health`) 0.0)
            (`self.Death`)))
        (:`then_1`
          ;[0.05127 0.05127 0.05127] Set percentage on HP bar, check if there is a progress bar on the owner first
          (bind _healthprogressbar (`self.HealthProgressBar`)
            (:`then`
              (`ProgressBar.SetPercent` _healthprogressbar (/ (`self.Health`) (`self.MaxHealth`))))
            (:`else`)))))))