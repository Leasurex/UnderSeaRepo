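; Player combat component providing target lock, punch combos, directional dodge, absorb, parry and a charge-consuming super punch.
; Target lock sphere-traces from the camera, attaches a marker and steers control rotation each tick, enabling strafing that gates absorb, parry and super punch.
; Actions play montages with state flags, and montage notifies end the punch combo unless attack was pressed again.
; A looping timer runs punch sphere traces, throttling damage with DoOnce and a delay.
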(event `self.ReceiveBeginPlay`
  ;[0.05127 0.05127 0.05127] When game begins, set player as player BP
  (bind _asbp_player_character (cast `/Game/Blueprints/BP_PlayerCharacter` (`self.GetOwner`)))
  (set `self.Player BP` _asbp_player_character))

(event `EnhancedInput|/Game/ThirdPerson/Input/Actions/IA_Lock`
  (params (ActionValue :type Boolean) (ElapsedSeconds :type "Float (double-precision)") (TriggeredSeconds :type "Float (double-precision)") (InputAction :type "InputAction Object Reference" :default "/Game/ThirdPerson/Input/Actions/IA_Lock.IA_Lock"))
  (bind _returnvalue (`Actor.GetTransform` (`self.TargetLockActor`)))
  (bind _transformcomponent (`PlayerCameraManager.TransformComponent` (`GameplayStatics.GetPlayerCameraManager` 0)))
  (bind _charactermovement (`Character.CharacterMovement` (`self.Player BP`)))
  (bind _charactermovement_2 (`Character.CharacterMovement` (`self.Player BP`)))
  (bind (_returnvalue_x _returnvalue_y _returnvalue_z) (`KismetMathLibrary.BreakVector` (`SceneComponent.K2_GetComponentLocation` _transformcomponent)))
  (bind _returnvalue_2 (`KismetMathLibrary.MakeVector` _returnvalue_x _returnvalue_y (+ _returnvalue_z 100.0)))
  ;[0.05127 0.05127 0.05127] Target Lock Mechanic
  (:`Started`
    ;;[0.05127 0.05127 0.05127] enable lock on if not already locked on to that enemy
    (`self.TargetLockActor`
      (:`then`
        ;;[0.05127 0.05127 0.05127] toggle target lock of if you click lock on again
        (set `self.TargetLockActor` null)
        ;;[0.05127 0.05127 0.05127] Allow player to move independently from the camera, (disable strafing)
        (set `CharacterMovementComponent.bOrientRotationToMovement` true _charactermovement)
        (set `CharacterMovementComponent.bUseControllerDesiredRotation` false _charactermovement)
        ;;[0.05127 0.05127 0.05127] Deletes the white dot when not targeting
        (`Actor.K2_DestroyActor` (`self.TargetLockWidget`)))
      (:`else`
        ;;[0.05127 0.05127 0.05127] big radius for our player to detect enemies
        (bind (_outhit _returnvalue_3) (`KismetSystemLibrary.SphereTraceSingleForObjects` :`Start` _returnvalue_2 :`End` (+ _returnvalue_2 (* (`KismetMathLibrary.GetForwardVector` (`SceneComponent.K2_GetComponentRotation` _transformcomponent)) 1750)) :`Radius` 150.0 :`ObjectTypes` (`|MakeArray` "ObjectTypeQuery3" :!type "EObjectTypeQuery Enum") :`DrawTime` 2.0))
        (if _returnvalue_3
          ;;[0.05127 0.05127 0.05127] when locked in, camera will always look at the enemy (enable strafing)
          (set `self.TargetLockActor` (`.HitActor` (`GameplayStatics.BreakHitResult` _outhit)))
          (set `CharacterMovementComponent.bOrientRotationToMovement` false _charactermovement_2)
          (set `CharacterMovementComponent.bUseControllerDesiredRotation` true _charactermovement_2)
          ;;[0.05127 0.05127 0.05127] Spawns the little white target lock widget on the enemy
          (bind _returnvalue_4 (`|SpawnActorFromClass` "/Game/Blueprints/BP_TargetLockWidget.BP_TargetLockWidget_C" (`KismetMathLibrary.MakeTransform` (`KismetMathLibrary.MakeVector` (.x (.location _returnvalue)) (.y (.location _returnvalue)) (+ (.z (.location _returnvalue)) 20.0)) (.rotation _returnvalue)) "AlwaysSpawn" "MultiplyWithRoot" null null))
          (bind _output_get (set `self.TargetLockWidget` _returnvalue_4))
          ;;[0.05127 0.05127 0.05127] Attach the target lock widget on the enemy
          (`Actor.K2_AttachToActor` _output_get (`self.TargetLockActor`) "None" "SnapToTarget" "SnapToTarget" "SnapToTarget" true))))))

(event `self.ReceiveTick`
  (params (DeltaSeconds :type "Float (single-precision)"))
  (bind (_returnvalue_roll _returnvalue_pitch _returnvalue_yaw) (`KismetMathLibrary.BreakRotator` (`KismetMathLibrary.FindLookAtRotation` (`Actor.K2_GetActorLocation` (`self.Player BP`)) (`Actor.K2_GetActorLocation` (`self.TargetLockActor`)))))
  ;[0.05127 0.05127 0.05127] Target Lock Mechanic
  ;;[0.05127 0.05127 0.05127] Target lock update. Every tick, make player camera look at the locked on enemy
  (`self.TargetLockActor`
    (:`then`
      (`Controller.SetControlRotation` (`Pawn.GetController` (`self.Player BP`)) (`KismetMathLibrary.MakeRotator` _returnvalue_roll (+ _returnvalue_pitch -20.0) _returnvalue_yaw)))
    (:`else`)))

(event `EnhancedInput|/Game/ThirdPerson/Input/Actions/IA_Attack`
  (params (ActionValue :type Boolean) (ElapsedSeconds :type "Float (double-precision)") (TriggeredSeconds :type "Float (double-precision)") (InputAction :type "InputAction Object Reference" :default "/Game/ThirdPerson/Input/Actions/IA_Attack.IA_Attack"))
  ;[0.05127 0.05127 0.05127] Punch Combo Animation
  (:`Started`
    ;;[0.05127 0.05127 0.05127] Check if player is not attacking already
    (if (not (`self.IsAttacking?`))
      ;;[0.05127 0.05127 0.05127] Stop player movement
      (`CharacterMovementComponent.SetMovementMode` (`Character.CharacterMovement` (`self.Player BP`)) "MOVE_None" 0)
      (set `self.IsAttacking?` true)
      ;;[0.05127 0.05127 0.05127] play basic attack
      (`|PlayMontage` (`Character.Mesh` (`self.Player BP`)) "/Game/CombatAnimations/Montage_PunchComboRoot.Montage_PunchComboRoot"
        (:`OnCompleted`
          ;;[0.05127 0.05127 0.05127] set attacking & combo to false if completed or interrupted
          (set `self.IsAttacking?` false :!label _label)
          (set `self.Combo?` false)
          ;[0.05127 0.05127 0.05127] Target Lock Mechanic
          ;;[0.05127 0.05127 0.05127] re-enable movement
          (`CharacterMovementComponent.SetMovementMode` (`Character.CharacterMovement` (`self.Player BP`)) "MOVE_Walking" 0))
        (:`OnInterrupted`
          (goto _label))
        (:`OnNotifyBegin`
          (if (and (`self.IsAttacking?`) (`self.Combo?`))
            ;;[0.05127 0.05127 0.05127] if you have combo, set combo back to false, you can proceed to follow the attack animation if you keep clicking, if you dont have combo then the montage would have stopped mid way and not play the entire attack
            (set `self.Combo?` false)
            (else
              ;;[0.05127 0.05127 0.05127] If no combo then stop attacking, this counts as an interrupt which will set comba and attacking to false
              (`AnimInstance.Montage_Stop` (`SkeletalMeshComponent.GetAnimInstance` (`Character.Mesh` (`self.Player BP`))) 0.3 "/Game/CombatAnimations/Montage_PunchComboRoot.Montage_PunchComboRoot")))))
      (else
        ;;[0.05127 0.05127 0.05127] if you are still attacking and you press the button, you will execute the next attack and have combo
        (set `self.Combo?` true)))))

(event `EndDamageTrace`
  ;[0.05127 0.05127 0.05127] Punch Trace
  (if (`KismetSystemLibrary.K2_IsValidTimerHandle` (stale `BeginDamageTrace` _returnvalue))
    (`KismetSystemLibrary.K2_ClearAndInvalidateTimerHandle` (stale `BeginDamageTrace` _returnvalue))))

(event `BeginDamageTrace`
  ;[0.05127 0.05127 0.05127] Punch Trace
  (bind _returnvalue (`KismetSystemLibrary.K2_SetTimerDelegate` (delegate `DamageTrace`) 0.01 true)))

(event `DamageTrace`
  (bind _mesh (`Character.Mesh` (`self.Player BP`)))
  (bind _returnvalue (`SceneComponent.K2_GetComponentLocation` _mesh))
  ;[0.05127 0.05127 0.05127] Punch Trace
  (bind (_outhit _returnvalue_2) (`KismetSystemLibrary.SphereTraceSingleForObjects` :`Start` (+ _returnvalue (0.0 0.0 100.0)) :`End` (+ (+ _returnvalue (* (`KismetMathLibrary.GetForwardVector` (`KismetMathLibrary.Conv_VectorToRotator` (`KismetMathLibrary.GreaterGreater_VectorRotator` (`KismetMathLibrary.Conv_RotatorToVector` (`SceneComponent.K2_GetComponentRotation` _mesh)) (struct :`Yaw` 90.0)))) 165)) (0.0 0.0 100.0)) :`Radius` 50.0 :`ObjectTypes` (`|MakeArray` "ObjectTypeQuery3" :!type "EObjectTypeQuery Enum") :`DrawTime` 1.0))
  (if _returnvalue_2
    ;;[0.05127 0.05127 0.05127] Since were running this every 0.01 sec, we need to only apply damage once and ad a delay
    (`/Engine/EditorBlueprintResources/StandardMacros.DoOnce` false :!label _label_2
      (:`Completed`
        (if (`self.IsSuperPunching?`)
          (bind _output_get (set `self.PunchDamage` 100.0))
          (bind (_bblockinghit _binitialoverlap _time _distance _location _impactpoint _normal _impactnormal _physmat _hitactor) (`GameplayStatics.BreakHitResult` _outhit))
          (`GameplayStatics.ApplyDamage` _hitactor _output_get)
          (else
            (bind _output_get_2 (set `self.PunchDamage` 5.0))
            (`GameplayStatics.ApplyDamage` _hitactor _output_get_2)))
        (`KismetSystemLibrary.Delay` 0.2)
        (goto _label_2 :!via `Reset`)))))

(event `EnhancedInput|/Game/ThirdPerson/Input/Actions/IA_Dodge`
  (params (ActionValue :type Boolean) (ElapsedSeconds :type "Float (double-precision)") (TriggeredSeconds :type "Float (double-precision)") (InputAction :type "InputAction Object Reference" :default "/Game/ThirdPerson/Input/Actions/IA_Dodge.IA_Dodge"))
  ;[0.05127 0.05127 0.05127] Dodge
  (:`Started`
    (if (not (`self.IsDodging?`))
      (set `self.IsDodging?` true)
      (`|ExecutionSequence`
        (:`then_0`
          ;;[0.05127 0.05127 0.05127] If the character is strafing, then
          (if (`CharacterMovementComponent.bUseControllerDesiredRotation` (`Character.CharacterMovement` (`self.Player BP`)))
            (switch `string` (`KismetTextLibrary.Conv_TextToString` (`KismetInputLibrary.Key_GetDisplayName` (`/Game/Blueprints/BP_PlayerCharacter.DirectionKey` (`self.Player BP`))))
              (:`W`
                (set `self.MovementDirection` "NewEnumerator0"))
              (:`A`
                (set `self.MovementDirection` "NewEnumerator1"))
              (:`S`
                (set `self.MovementDirection` "NewEnumerator2"))
              (:`D`
                (set `self.MovementDirection` "NewEnumerator3")))
            (else
              ;;[0.05127 0.05127 0.05127] If not strafing then use forward dodge
              (set `self.MovementDirection` "NewEnumerator0"))))
        (:`then_1`
          ;;[0.05127 0.05127 0.05127] Wait for Dodge animation to finish to do another dodge, so you cant spam dodge
          (`|PlayMontage` (`Character.Mesh` (`self.Player BP`)) (select `/Game/Blueprints/E_MovementDirection` (`self.MovementDirection`) :`NewEnumerator0` "/Game/CombatAnimations/Dodge/Montage_DodgeForwardRoot.Montage_DodgeForwardRoot" :`NewEnumerator1` "/Game/CombatAnimations/Dodge/Montage_DodgeLeftRoot.Montage_DodgeLeftRoot" :`NewEnumerator2` "/Game/CombatAnimations/Dodge/Montage_DodgeBackwardRoot.Montage_DodgeBackwardRoot" :`NewEnumerator3` "/Game/CombatAnimations/Dodge/Montage_DodgeRightRoot.Montage_DodgeRightRoot" :!type "AnimMontage Object Reference")
            (:`OnCompleted`
              _)
            (:`OnInterrupted`
              _))
          (set `self.IsDodging?` false))))))

(event `Key|RightMouseButton`
  (params (Key :type "Key Structure"))
  ;[0.05127 0.05127 0.05127] Absorb
  (:`Pressed`
    (if (not (`self.IsBlocking?`))
      (if (`CharacterMovementComponent.bUseControllerDesiredRotation` (`Character.CharacterMovement` (`self.Player BP`)))
        (`CharacterMovementComponent.SetMovementMode` (`Character.CharacterMovement` (`self.Player BP`)) "MOVE_None" 0)
        (set `self.IsBlocking?` true)
        (`|PlayMontage` (`Character.Mesh` (`self.Player BP`)) "/Game/CombatAnimations/Montage_AbsorbIdle.Montage_AbsorbIdle"
          (:`then`
            (`KismetSystemLibrary.PrintString` "Absorbing"))
          (:`OnCompleted`
            (set `self.IsBlocking?` false :!label _label_3)
            (`CharacterMovementComponent.SetMovementMode` (`Character.CharacterMovement` (`self.Player BP`)) "MOVE_Walking" 0))
          (:`OnInterrupted`
            (goto _label_3))))))
  (:`Released`
    (set `self.IsBlocking?` false)
    (`AnimInstance.Montage_Stop` (`SkeletalMeshComponent.GetAnimInstance` (`Character.Mesh` (`self.Player BP`))) 0.3 "/Game/CombatAnimations/Montage_AbsorbIdle.Montage_AbsorbIdle")))

(event `EnhancedInput|/Game/ThirdPerson/Input/Actions/IA_Parry`
  (params (ActionValue :type Boolean) (ElapsedSeconds :type "Float (double-precision)") (TriggeredSeconds :type "Float (double-precision)") (InputAction :type "InputAction Object Reference" :default "/Game/ThirdPerson/Input/Actions/IA_Parry.IA_Parry"))
  ;[0.05127 0.05127 0.05127] Parry
  (:`Triggered`
    (if (not (`self.IsParrying?`))
      (if (`CharacterMovementComponent.bUseControllerDesiredRotation` (`Character.CharacterMovement` (`self.Player BP`)))
        (`CharacterMovementComponent.SetMovementMode` (`Character.CharacterMovement` (`self.Player BP`)) "MOVE_None" 0)
        (set `self.IsParrying?` true)
        (`|PlayMontage` (`Character.Mesh` (`self.Player BP`)) "/Game/CombatAnimations/Montage_Parry.Montage_Parry"
          (:`then`
            (`KismetSystemLibrary.PrintString` "Parrying"))
          (:`OnCompleted`
            (set `self.IsParrying?` false :!label _label_4)
            (`CharacterMovementComponent.SetMovementMode` (`Character.CharacterMovement` (`self.Player BP`)) "MOVE_Walking" 0))
          (:`OnInterrupted`
            (goto _label_4)))))))

(event `EnhancedInput|/Game/ThirdPerson/Input/Actions/IA_SuperPunch`
  (params (ActionValue :type Boolean) (ElapsedSeconds :type "Float (double-precision)") (TriggeredSeconds :type "Float (double-precision)") (InputAction :type "InputAction Object Reference" :default "/Game/ThirdPerson/Input/Actions/IA_SuperPunch.IA_SuperPunch"))
  ;[0.05127 0.05127 0.05127] Super Punch
  (:`Started`
    (if (> (`/Game/Blueprints/BPC_Stats.Charge` (`/Game/Blueprints/BP_PlayerCharacter.BPC_Stats` (`self.Player BP`))) 0.0)
      (if (`CharacterMovementComponent.bUseControllerDesiredRotation` (`Character.CharacterMovement` (`self.Player BP`)))
        (`CharacterMovementComponent.SetMovementMode` (`Character.CharacterMovement` (`self.Player BP`)) "MOVE_None" 0)
        (set `self.IsSuperPunching?` true)
        (`/Game/Blueprints/BPC_Stats.IncreaseCharge` (`/Game/Blueprints/BP_PlayerCharacter.BPC_Stats` (`self.Player BP`)) "NewEnumerator1" -1.0)
        (`|PlayMontage` (`Character.Mesh` (`self.Player BP`)) "/Game/CombatAnimations/Montage_SuperPunch.Montage_SuperPunch"
          (:`OnCompleted`
            _)
          (:`OnInterrupted`
            _))
        (set `self.IsSuperPunching?` false)
        (`CharacterMovementComponent.SetMovementMode` (`Character.CharacterMovement` (`self.Player BP`)) "MOVE_Walking" 0)))))