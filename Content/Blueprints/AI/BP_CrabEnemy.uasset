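; Crab enemy character with punch, kick and chop montage attacks, a widget health bar, and damage routed into its stats component.
; Begin/End events run looping timers that sphere-trace ahead, with DoOnce and delays limiting repeat hits.
; A blocking player absorbs kicks for charge, a parrying player stuns the crab on chops, and otherwise damage applies.
; Death ragdolls the crab, zeroes the player's walk speed, calls CrabDeath and destroys the actor after a delay.
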(event `self.ReceiveBeginPlay`
  (bind _aswbp_enemy_health_bar (cast `/Game/UI/WBP_EnemyHealthBar` (`WidgetComponent.GetWidget` (`self.Widget`))))
  (`/Game/Blueprints/BPC_Stats.SetHealthProgressBar` (`self.BPC_Stats`) (`/Game/UI/WBP_EnemyHealthBar.HealthBar` _aswbp_enemy_health_bar)))

(event `self.ReceiveAnyDamage`
  (params (Damage :type "Float (single-precision)") (DamageType :type "DamageType Object Reference") (InstigatedBy :type "Controller Object Reference") (DamageCauser :type "Actor Object Reference"))
  (`/Game/Blueprints/BPC_Stats.IncreaseValue` (`self.BPC_Stats`) "NewEnumerator0" (* Damage -1.0)))

(event `/Game/Blueprints/BPI_Damage.EndPunchTrace`
  ;[0.05127 0.05127 0.05127] Punch Trace
  (if (`KismetSystemLibrary.K2_IsValidTimerHandle` (stale `/Game/Blueprints/BPI_Damage.BeginPunchTrace` _returnvalue))
    (`KismetSystemLibrary.K2_ClearAndInvalidateTimerHandle` (stale `/Game/Blueprints/BPI_Damage.BeginPunchTrace` _returnvalue))))

(event `/Game/Blueprints/BPI_Damage.BeginPunchTrace`
  ;[0.05127 0.05127 0.05127] Punch Trace
  (bind _returnvalue (`KismetSystemLibrary.K2_SetTimerDelegate` (delegate `DamageTrace`) 0.01 true)))

(event `DamageTrace`
  (bind _mesh (`self.Mesh`))
  (bind _returnvalue (`SceneComponent.K2_GetComponentLocation` _mesh))
  ;[0.05127 0.05127 0.05127] Punch Trace
  ;;[0.05127 0.05127 0.05127] Check if still alive, (cuz it can still attack when dead)
  (if (not (`self.IsDead?`))
    (bind (_outhit _returnvalue_2) (`KismetSystemLibrary.SphereTraceSingleForObjects` :`Start` (+ _returnvalue (0.0 0.0 100.0)) :`End` (+ (+ _returnvalue (* (`KismetMathLibrary.GetForwardVector` (`KismetMathLibrary.Conv_VectorToRotator` (`KismetMathLibrary.GreaterGreater_VectorRotator` (`KismetMathLibrary.Conv_RotatorToVector` (`SceneComponent.K2_GetComponentRotation` _mesh)) (struct :`Yaw` 90.0)))) 165)) (0.0 0.0 100.0)) :`Radius` 50.0 :`ObjectTypes` (`|MakeArray` "ObjectTypeQuery3" :!type "EObjectTypeQuery Enum") :`DrawDebugType` "ForOneFrame" :`DrawTime` 1.0))
    (if _returnvalue_2
      ;;[0.05127 0.05127 0.05127] Since were running this every 0.01 sec, we need to only apply damage once and ad a delay
      (`/Engine/EditorBlueprintResources/StandardMacros.DoOnce` false :!label _label
        (:`Completed`
          (`GameplayStatics.ApplyDamage` (`.HitActor` (`GameplayStatics.BreakHitResult` _outhit)) (`self.PunchDamage`))
          (`KismetSystemLibrary.Delay` 0.8)
          (goto _label :!via `Reset`))))))

(event `/Game/Blueprints/BPI_Damage.Death`
  ;[0.05127 0.05127 0.05127] Death
  (`CharacterMovementComponent.DisableMovement` (`self.CharacterMovement`))
  (`PrimitiveComponent.SetSimulatePhysics` (`self.Mesh`) true)
  (set `self.IsDead?` true)
  (bind _asbp_player_character (cast `/Game/Blueprints/BP_PlayerCharacter` (`GameplayStatics.GetPlayerCharacter` 0)))
  (set `CharacterMovementComponent.MaxWalkSpeed` 0.0 (`Character.CharacterMovement` _asbp_player_character))
  (`self.CrabDeath`)
  (`KismetSystemLibrary.Delay` 5.0)
  (`self.K2_DestroyActor`))

(event `/Game/Blueprints/BPI_Damage.EndAbsorbWindow`
  ;[0.05127 0.05127 0.05127] Kick Absorb
  (if (`KismetSystemLibrary.K2_IsValidTimerHandle` (stale `/Game/Blueprints/BPI_Damage.BeginAbsorbWindow` _returnvalue))
    (`KismetSystemLibrary.K2_ClearAndInvalidateTimerHandle` (stale `/Game/Blueprints/BPI_Damage.BeginAbsorbWindow` _returnvalue))))

(event `/Game/Blueprints/BPI_Damage.BeginAbsorbWindow`
  ;[0.05127 0.05127 0.05127] Kick Absorb
  (bind _returnvalue (`KismetSystemLibrary.K2_SetTimerDelegate` (delegate `AbsorbWindow`) 0.01 true)))

(event `AbsorbWindow`
  (bind _mesh (`self.Mesh`))
  (bind _returnvalue (`SceneComponent.K2_GetComponentLocation` _mesh))
  ;[0.05127 0.05127 0.05127] Kick Absorb
  ;;[0.05127 0.05127 0.05127] Check if still alive, (cuz it can still attack when dead)
  (if (not (`self.IsDead?`))
    (bind (_outhit _returnvalue_2) (`KismetSystemLibrary.SphereTraceSingleForObjects` :`Start` (+ _returnvalue (0.0 0.0 100.0)) :`End` (+ (+ _returnvalue (* (`KismetMathLibrary.GetForwardVector` (`KismetMathLibrary.Conv_VectorToRotator` (`KismetMathLibrary.GreaterGreater_VectorRotator` (`KismetMathLibrary.Conv_RotatorToVector` (`SceneComponent.K2_GetComponentRotation` _mesh)) (struct :`Yaw` 90.0)))) 185)) (0.0 0.0 100.0)) :`Radius` 50.0 :`ObjectTypes` (`|MakeArray` "ObjectTypeQuery3" :!type "EObjectTypeQuery Enum") :`DrawDebugType` "ForOneFrame" :`DrawTime` 1.0))
    (if _returnvalue_2
      (bind (_bblockinghit _binitialoverlap _time _distance _location _impactpoint _normal _impactnormal _physmat _hitactor) (`GameplayStatics.BreakHitResult` _outhit))
      (bind _asbp_player_character (cast `/Game/Blueprints/BP_PlayerCharacter` _hitactor))
      (`/Engine/EditorBlueprintResources/StandardMacros.DoOnce` false :!label _label_2
        (:`Completed`
          ;;[0.05127 0.05127 0.05127] Check if player is absorbing
          (if (`/Game/Blueprints/BPC_Combat.IsBlocking?` (`/Game/Blueprints/BP_PlayerCharacter.BPC_Combat` _asbp_player_character))
            ;;[0.05127 0.05127 0.05127] Since were running this every 0.01 sec add delay
            (`KismetSystemLibrary.PrintString` "ABSORBED!!!")
            (`|PlayMontage` (`Character.Mesh` _asbp_player_character) "/Game/CombatAnimations/Montage_AbsorbSuccess.Montage_AbsorbSuccess" 1.25
              (:`then`
                (`/Game/Blueprints/BPC_Stats.IncreaseCharge` (`/Game/Blueprints/BP_PlayerCharacter.BPC_Stats` _asbp_player_character) "NewEnumerator1" 1.0)
                (`KismetSystemLibrary.Delay` 0.5)
                (goto _label_2 :!via `Reset`)))
            (else
              ;;[0.05127 0.05127 0.05127] Since were running this every 0.01 sec, we need to only apply damage once and add a delay
              (`GameplayStatics.ApplyDamage` _hitactor (`self.PunchDamage`))
              (`KismetSystemLibrary.Delay` 0.5)
              (goto _label_2 :!via `Reset`))))))))

(event `/Game/Blueprints/BPI_Damage.EndParryWindow`
  ;[0.05127 0.05127 0.05127] Chop Parry
  (if (`KismetSystemLibrary.K2_IsValidTimerHandle` (stale `/Game/Blueprints/BPI_Damage.BeginParryWindow` _returnvalue))
    (`KismetSystemLibrary.K2_ClearAndInvalidateTimerHandle` (stale `/Game/Blueprints/BPI_Damage.BeginParryWindow` _returnvalue))))

(event `/Game/Blueprints/BPI_Damage.BeginParryWindow`
  ;[0.05127 0.05127 0.05127] Chop Parry
  (bind _returnvalue (`KismetSystemLibrary.K2_SetTimerDelegate` (delegate `ParryWindow`) 0.01 true)))

(event `ParryWindow`
  (bind _mesh (`self.Mesh`))
  (bind _charactermovement (`self.CharacterMovement`))
  (bind _returnvalue (`SceneComponent.K2_GetComponentLocation` _mesh))
  ;[0.05127 0.05127 0.05127] Chop Parry
  ;;[0.05127 0.05127 0.05127] Check if still alive, (cuz it can still attack when dead)
  (if (not (`self.IsDead?`))
    (bind (_outhit _returnvalue_2) (`KismetSystemLibrary.SphereTraceSingleForObjects` :`Start` (+ _returnvalue (0.0 0.0 100.0)) :`End` (+ (+ _returnvalue (* (`KismetMathLibrary.GetForwardVector` (`KismetMathLibrary.Conv_VectorToRotator` (`KismetMathLibrary.GreaterGreater_VectorRotator` (`KismetMathLibrary.Conv_RotatorToVector` (`SceneComponent.K2_GetComponentRotation` _mesh)) (struct :`Yaw` 90.0)))) 165)) (0.0 0.0 100.0)) :`Radius` 50.0 :`ObjectTypes` (`|MakeArray` "ObjectTypeQuery3" :!type "EObjectTypeQuery Enum") :`DrawDebugType` "ForOneFrame" :`DrawTime` 1.0))
    (if _returnvalue_2
      (bind (_bblockinghit _binitialoverlap _time _distance _location _impactpoint _normal _impactnormal _physmat _hitactor) (`GameplayStatics.BreakHitResult` _outhit))
      (bind _asbp_player_character (cast `/Game/Blueprints/BP_PlayerCharacter` _hitactor))
      (`/Engine/EditorBlueprintResources/StandardMacros.DoOnce` false :!label _label_3
        (:`Completed`
          ;;[0.05127 0.05127 0.05127] Check if player is Parrying
          (if (`/Game/Blueprints/BPC_Combat.IsParrying?` (`/Game/Blueprints/BP_PlayerCharacter.BPC_Combat` _asbp_player_character))
            (set `self.IsParried?` true)
            ;;[0.05127 0.05127 0.05127] Since were running this every 0.01 sec add delay
            (`KismetSystemLibrary.PrintString` "PARRIED!!!")
            (`|PlayMontage` (`self.Mesh`) "/Game/Enemies/Crab/Animations/Montage_CrabStunned.Montage_CrabStunned"
              (:`then`
                (set `CharacterMovementComponent.MaxWalkSpeed` 0.0 _charactermovement)
                (`KismetSystemLibrary.Delay` 0.5)
                (set `self.IsParried?` false)
                (goto _label_3 :!via `Reset`))
              (:`OnCompleted`
                _)
              (:`OnInterrupted`
                _))
            (set `CharacterMovementComponent.MaxWalkSpeed` 280.0 _charactermovement)
            (else
              ;;[0.05127 0.05127 0.05127] Since were running this every 0.01 sec, we need to only apply damage once and add a delay
              (`GameplayStatics.ApplyDamage` _hitactor (`self.PunchDamage`))
              (`KismetSystemLibrary.Delay` 0.5)
              (goto _label_3 :!via `Reset`))))))))

(fn `ChopAttack`
  (returns (Duration :type "Float (double-precision)"))
  (bind _returnvalue (`self.PlayAnimMontage` "/Game/Enemies/Crab/Animations/Montage_CrabChop.Montage_CrabChop"))
  (return _returnvalue))

(fn `KickAttack`
  (returns (Duration :type "Float (double-precision)"))
  (bind _returnvalue (`self.PlayAnimMontage` "/Game/Enemies/Crab/Animations/Montage_CrabKick.Montage_CrabKick"))
  (return _returnvalue))

(fn `PunchAttack`
  (returns (Duration :type "Float (double-precision)"))
  (bind _returnvalue (`self.PlayAnimMontage` "/Game/Enemies/Crab/Animations/Montage_CrabPunch.Montage_CrabPunch"))
  (return _returnvalue))

(fn `UserConstructionScript`)